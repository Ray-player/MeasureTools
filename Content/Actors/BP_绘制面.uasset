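; BP_绘制面 is an actor for drawing polygon areas in the world and displaying their measured area.
; Left clicks trace under the cursor and add point widgets to WBP_AreaMainUI, slightly above the hit.
; Right click disables input and, given at least three points, triangulates them into a procedural mesh section with winding-based vertical normals.
; It then labels the scaled polygon area and creates a fresh UI for the next shape.
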(event Custom|启用控制输入
  (params (启用 :type Boolean))
  (if 启用
    (Input|EnableInput (Game|GetPlayerController 0))
    (else
      (Input|DisableInput (Game|GetPlayerController 0)))))

(event EventBeginPlay
  (bind _returnvalue (UserInterface|CreateWidget "/MeasureTools/Widget/WBP_AreaMainUI.WBP_AreaMainUI_C"))
  (bind _output_get (Variables|Default|SetMainUI _returnvalue))
  (UserInterface|Viewport|AddtoViewport _output_get 0)
  (CallFunction|启用控制输入 true))

(event Input|MouseEvents|RightMouseButton
  (params (Key :type Key%20Structure))
  (:Pressed
    (CallFunction|启用控制输入 false)
    (if (>= (Utilities|Array|Length (Variables|/MeasureTools/Widget/WBP_AreaMainUI.WBP_AreaMainUI_C|GetVectorArray (Variables|Default|GetMainUI))) 3)
      (Default|结束绘制停用移动点位 (Variables|Default|GetMainUI))
      (bind _triangles (CallFunction|TriangulatePolygon (Variables|/MeasureTools/Widget/WBP_AreaMainUI.WBP_AreaMainUI_C|GetVectorArray (Variables|Default|GetMainUI))))
      (Class|ProceduralMeshComponent|CreateMeshSectionLinearColor (Variables|Default|GetProceduralMesh) (Variables|Default|GetSection%20Index) (Variables|/MeasureTools/Widget/WBP_AreaMainUI.WBP_AreaMainUI_C|GetVectorArray (Variables|Default|GetMainUI)) _triangles (CallFunction|计算法线 (> (CallFunction|CalculatePoligonArea _triangles (Variables|/MeasureTools/Widget/WBP_AreaMainUI.WBP_AreaMainUI_C|GetVectorArray (Variables|Default|GetMainUI))) 0.0)) 0 0 0 0 0 0 false)
      (Rendering|Material|SetMaterial (Variables|Default|GetProceduralMesh) (Variables|Default|GetSection%20Index) "/MeasureTools/Mat/M_Color_Inst.M_Color_Inst")
      (Math|Integer|IncrementInt (Variables|Default|GetSection%20Index)
        (:%20%20
          (Utilities|FlowControl|Sequence
            (:then_0
              (Utilities|IsValid (Variables|Default|GetMainUI)
                (:Is%20Valid
                  (bind _returnvalue (UserInterface|CreateWidget "/MeasureTools/Widget/WBP_Text.WBP_Text_C"))
                  (Default|设置文本 _returnvalue (Utilities|Text|FormatText "{S}/m2" (Utilities|Text|ToText(Float) (/ (Math|Float|Absolute(Float) (CallFunction|CalculatePoligonArea _triangles (Variables|/MeasureTools/Widget/WBP_AreaMainUI.WBP_AreaMainUI_C|GetVectorArray (Variables|Default|GetMainUI)))) 1e+02) "HalfToEven")))
                  (Default|设置面积文本 (Variables|Default|GetMainUI) _returnvalue))))
            (:then_1
              (bind _returnvalue_2 (UserInterface|CreateWidget "/MeasureTools/Widget/WBP_AreaMainUI.WBP_AreaMainUI_C"))
              (bind _output_get (Variables|Default|SetMainUI _returnvalue_2))
              (UserInterface|Viewport|AddtoViewport _output_get 0))))))))

(event Input|MouseEvents|LeftMouseButton
  (params (Key :type Key%20Structure))
  (bind _returnvalue (Game|GetPlayerController 0))
  (bind (_worldlocation _worlddirection) (Game|Player|ConvertMouseLocationToWorldSpace _returnvalue))
  (:Pressed
    (bind (_outhit _returnvalue_2) (Collision|LineTraceByChannel _worldlocation (+ _worldlocation (* _worlddirection 1e+06)) "TraceTypeQuery1" false 0 "None"))
    (if _returnvalue_2
      (bind _returnvalue_3 (UserInterface|CreateWidget "/MeasureTools/Widget/WBP_AreaPoint.WBP_AreaPoint_C" 0 (Variables|Default|GetMainUI)))
      (Default|添加点 (Variables|Default|GetMainUI) (Math|Vector|MakeVector (.X (Math|Vector|BreakVector (.Location (Collision|BreakHitResult _outhit)))) (.Y (Math|Vector|BreakVector (.Location (Collision|BreakHitResult _outhit)))) (+ (.Z (Math|Vector|BreakVector (.Location (Collision|BreakHitResult _outhit)))) 1.0)) _returnvalue_3))))

(fn ConstructionScript)

(fn 计算法线
  (params (顺时针 :type Boolean))
  (bind _output_get (LocalVariables|SetNormal (Variables|/MeasureTools/Widget/WBP_AreaMainUI.WBP_AreaMainUI_C|GetVectorArray (Variables|Default|GetMainUI))))
  (for (_ _array_index) _output_get
    (Utilities|Array|SetArrayElem _output_get _array_index (select 顺时针 (Math|Vector|MakeVector 0.0 0.0 -1.0) (Math|Vector|MakeVector 0.0 0.0 1.0))))
  (return (LocalVariables|GetNormal)))