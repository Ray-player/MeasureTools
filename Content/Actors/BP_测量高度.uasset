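; BP_测量高度 is a height-measurement tool actor that lets the player mark scene points with mouse clicks.
; On BeginPlay it adds a WBP_HeightMainUI to the viewport and enables its own input.
; Left click line-traces under the cursor, passes the hit and a new WBP_HeightPoint to that UI, then opens a fresh UI for single-segment mode.
; Right click disables the actor's input, ending measurement.
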(event Custom|启用控制输入
  (params (启用 :type Boolean))
  (if 启用
    (Input|EnableInput (Game|GetPlayerController 0))
    (else
      (Input|DisableInput (Game|GetPlayerController 0)))))

(event EventBeginPlay
  (bind _returnvalue (UserInterface|CreateWidget "/MeasureTools/Widget/WBP_HeightMainUI.WBP_HeightMainUI_C"))
  (bind _output_get (Variables|Default|SetHeightMainUI _returnvalue))
  (UserInterface|Viewport|AddtoViewport _output_get 0)
  (CallFunction|启用控制输入 true))

(event Input|MouseEvents|RightMouseButton
  (params (Key :type Key%20Structure :default "None"))
  (:Pressed
    (CallFunction|启用控制输入 false)))

(event Input|MouseEvents|LeftMouseButton
  (params (Key :type Key%20Structure :default "None"))
  (bind _returnvalue (Game|GetPlayerController 0))
  (bind (_worldlocation _worlddirection) (Game|Player|ConvertMouseLocationToWorldSpace _returnvalue))
  (:Pressed
    (bind (_outhit _returnvalue_2) (Collision|LineTraceByChannel _worldlocation (+ _worldlocation (* _worlddirection 1e+06)) "TraceTypeQuery1" false 0 "None"))
    (if _returnvalue_2
      (bind _returnvalue_3 (UserInterface|CreateWidget "/MeasureTools/Widget/WBP_HeightPoint.WBP_HeightPoint_C" 0 (Variables|Default|GetHeightMainUI)))
      (Default|添加点 (Variables|Default|GetHeightMainUI) (.Location (Collision|BreakHitResult _outhit)) _returnvalue_3)
      ;[1 1 1] 单个线段绘制模式
      (bind _returnvalue_4 (UserInterface|CreateWidget "/MeasureTools/Widget/WBP_HeightMainUI.WBP_HeightMainUI_C"))
      (bind _output_get (Variables|Default|SetHeightMainUI _returnvalue_4))
      (UserInterface|Viewport|AddtoViewport _output_get 0))))

(fn ConstructionScript)